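; Health component that tracks an owning actor's current and maximum health.
; Inithealth sets both values, and DecreaseHealth subtracts damage down to zero, firing the update dispatcher and then the death dispatcher at zero.
; IncreaseHealth sets Health to the passed value capped at MaxHealth, without adding current Health, then fires the update dispatcher.
; Getters expose both values, while debug print chains are left unconnected.
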(fn `DecreaseHealth`
  (params (Value :type "Float (double-precision)"))
  (bind _health (`self.Health`))
  (if (> _health 0.0)
    (bind _output_get (set `self.Health` (`KismetMathLibrary.FMax` (- _health Value))))
    (`self.OnUpdateHealth` _output_get)
    (if (<= (`self.Health`) 0.0)
      (`self.OnDie`))))

(fn `GetHealth`
  (returns (Health :type "Float (double-precision)"))
  (return (`self.Health`)))

(fn `GetMaxHealth`
  (returns (MaxHealth :type "Float (double-precision)"))
  (return (`self.MaxHealth`)))

(fn `IncreaseHealth`
  (params (Value :type "Float (double-precision)"))
  (set `self.Health` (`KismetMathLibrary.FMin` (+ Value 0.0) (`self.MaxHealth`)))
  (`self.OnUpdateHealth` (`self.Health`)))

(fn `Inithealth`
  (params (`Max Health` :type "Float (double-precision)"))
  (bind _output_get (set `self.MaxHealth` `Max Health`))
  (set `self.Health` _output_get))