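; BP_Barrel is a destructible barrel actor that takes damage and is destroyed when its health runs out.
; A BPC health component is initialised on BeginPlay, and AnyDamage passes incoming damage straight to it.
; The component's update and death events are bound back to the barrel, which prints the new health, then on death prints a message and destroys itself.
; The cube's hit event is empty.
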(event `self.ReceiveBeginPlay`
  (`parent.ReceiveBeginPlay`)
  (`/Game/Bluprint/Component/BPC_HealthComponent.Inithealth` (`self.BPC_HealthComponent`) 100.0)
  (add `/Game/Bluprint/Component/BPC_HealthComponent.OnUpdateHealth` (`self.BPC_HealthComponent`) (delegate `OnHealthUpdated`))
  (add `/Game/Bluprint/Component/BPC_HealthComponent.OnDie` (`self.BPC_HealthComponent`) (delegate `OnOwnerDie`)))

(event `self.ReceiveAnyDamage`
  (params (Damage :type "Float (single-precision)") (DamageType :type "DamageType Object Reference") (InstigatedBy :type "Controller Object Reference") (DamageCauser :type "Actor Object Reference"))
  (`/Game/Bluprint/Component/BPC_HealthComponent.DecreaseHealth` (`self.BPC_HealthComponent`) Damage))

(event `self.Cube.OnComponentHit`
  (params (HitComponent :type "PrimitiveComponent Object Reference") (OtherActor :type "Actor Object Reference") (OtherComp :type "PrimitiveComponent Object Reference") (NormalImpulse :type "Vector Structure") (Hit :type "HitResult Structure (by ref)")))

(event `OnHealthUpdated`
  (params (NewHealth :type "Float (double-precision)"))
  (`KismetSystemLibrary.PrintText` (`|FormatText` (`KismetTextLibrary.Conv_DoubleToText` NewHealth "HalfToEven"))))

(event `OnOwnerDie`
  (`KismetSystemLibrary.PrintText` (`|FormatText` "{Owner}:Die" self))
  (`self.K2_DestroyActor`))

(fn `UserConstructionScript`)