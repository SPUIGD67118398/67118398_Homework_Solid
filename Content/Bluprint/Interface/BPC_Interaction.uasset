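; Player character component that detects nearby interactable actors, shows a screen-space prompt and triggers interaction.
; Each tick, a sphere trace around the owner maintains FoundInteract, which takes new actors only when empty.
; The "closest" target is the first listed actor within a view-angle cone, not the nearest, and positions the prompt widget and sets its text.
; Interact messages the first in-view actor, then removes it from the list.
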(event `self.ReceiveBeginPlay`
  (bind _interactwidgetcomp (`self.InteractWidgetComp`))
  (bind _asbp_player_character (cast `/Game/Bluprint/ThirdPerson/Blueprints/BP_Player_Character` (`self.GetOwner`)))
  (bind _output_get (set `self.OwnerCharacter` _asbp_player_character))
  (bind _returnvalue (`|AddComponentByClass` _output_get "/Script/UMG.WidgetComponent" true (`KismetMathLibrary.MakeTransform` (0.0 0.0 0.0))))
  (set `self.InteractWidgetComp` _returnvalue)
  (`|ExecutionSequence`
    (:`then_0`
      (`WidgetComponent.SetDrawSize` _interactwidgetcomp (400.0 50.0))
      (`WidgetComponent.SetWidgetSpace` _interactwidgetcomp "Screen"))
    (:`then_1`
      (bind _returnvalue_2 (`|CreateWidget` "/Game/Bluprint/Widgets/WBP_Interact.WBP_Interact_C"))
      (bind _output_get_2 (set `self.InteractWidget` _returnvalue_2))
      (`Widget.SetVisibility` _output_get_2 "Collapsed"))
    (:`then_2`
      (`WidgetComponent.SetWidget` (`self.InteractWidgetComp`) (`self.InteractWidget`)))))

(event `self.ReceiveTick`
  (params (DeltaSeconds :type "Float (single-precision)"))
  (bind _closestinteractable (`self.Closestinteractable`))
  (`/Engine/EditorBlueprintResources/StandardMacros.IsValid` (`self.OwnerCharacter`)
    (:`Is Valid`
      (`|ExecutionSequence`
        (:`then_0`
          (`self.FindInteractble`))
        (:`then_1`
          (bind _returnclosestinteractable (`self.FindClosesInteractable`))
          (`/Engine/EditorBlueprintResources/StandardMacros.IsValid` _returnclosestinteractable
            (:`Is Valid`
              (if (!= (`self.Closestinteractable`) _returnclosestinteractable)
                (set `self.Closestinteractable` _returnclosestinteractable)
                (`|ExecutionSequence`
                  (:`then_0`
                    (`Widget.SetVisibility` (`self.InteractWidget`) "Visible"))
                  (:`then_1`
                    (bind _returnvector (message `/Game/Bluprint/Interface/BPI_Interactable.GetInteractTextLocation` _closestinteractable))
                    (`SceneComponent.K2_SetWorldLocation` (`self.InteractWidgetComp`) _returnvector false false)
                    (bind _returntext (message `/Game/Bluprint/Interface/BPI_Interactable.GetInteractText` _closestinteractable))
                    (`/Game/Bluprint/Widgets/WBP_Interact.SetIneractText` (`self.InteractWidget`) _returntext)))))
            (:`Is Not Valid`
              (set `self.Closestinteractable` null)
              (`Widget.SetVisibility` (`self.InteractWidget`) "Collapsed"))))))))

(fn `FindClosesInteractable`
  (returns (ReturnClosestInteractable :type "Actor Object Reference"))
  (bind _found_interact (`self.Found Interact`))
  (if (`KismetArrayLibrary.Array_IsNotEmpty` _found_interact)
    (for _array_element _found_interact
      (if (`self.IsInteractTablenViewLength` _array_element)
        (return _array_element))))
  (return null))

(fn `FindInteractble`
  (locals (Timplnteractbles :type "Array of Actor Object Reference"))
  (bind _found_interact (`self.Found Interact`))
  (bind _returnvalue (`Actor.K2_GetActorLocation` (`self.GetOwner`)))
  (bind (_outhits _returnvalue_2) (`KismetSystemLibrary.SphereTraceMulti` _returnvalue _returnvalue 250.0 "TraceTypeQuery1"))
  (if _returnvalue_2
    ; Add Timp Interactables
    (for _array_element _outhits
      (bind (_bblockinghit _binitialoverlap _time _distance _location _impactpoint _normal _impactnormal _physmat _hitactor) (`GameplayStatics.BreakHitResult` _array_element))
      (bind _return_is_can (message `/Game/Bluprint/Interface/BPI_Interactable.CanInteractable` _hitactor))
      (if (and _bblockinghit _return_is_can)
        (`KismetArrayLibrary.Array_Add` (`local.Timplnteractbles`) _hitactor)))
    (if (`KismetArrayLibrary.Array_IsEmpty` (`self.Found Interact`))
      (`KismetArrayLibrary.Array_Append` (`self.Found Interact`) (`local.Timplnteractbles`))
      (else
        (bind (_arrayindex _arrayelement) (`/Engine/EditorBlueprintResources/StandardMacros.ReverseForEachLoop` _found_interact)
          (:`LoopBody`
            (if (not (`KismetArrayLibrary.Array_Contains` (`local.Timplnteractbles`) _arrayelement))
              (`KismetArrayLibrary.Array_RemoveItem` _found_interact _arrayelement))))))
    (else
      (`KismetArrayLibrary.Array_Clear` (`self.Found Interact`)))))

(fn `Interact`
  (locals (TmpInteractable :type "Actor Object Reference"))
  (bind _found_interact (`self.Found Interact`))
  (bind _tmpinteractable (`local.TmpInteractable`))
  (if (`KismetArrayLibrary.Array_IsNotEmpty` _found_interact)
    (for _array_element _found_interact
      (if (`self.IsInteractTablenViewLength` _array_element)
        (set `local.TmpInteractable` _array_element)
        (break)))
    (`/Engine/EditorBlueprintResources/StandardMacros.IsValid` _tmpinteractable
      (:`Is Valid`
        (`|ExecutionSequence`
          (:`then_0`
            (message `/Game/Bluprint/Interface/BPI_Interactable.Oninteract` _tmpinteractable (`self.OwnerCharacter`)))
          (:`then_1`
            (`KismetArrayLibrary.Array_RemoveItem` (`self.Found Interact`) _tmpinteractable)))))))

(fn `IsInteractTablenViewLength`
  (params (Interactble :type "Actor Object Reference"))
  (returns (ReturnValue :type Boolean))
  (return (<= (`KismetMathLibrary.DegAcos` (`KismetMathLibrary.Dot_VectorVector` (`KismetMathLibrary.GetForwardVector` (`Pawn.GetControlRotation` (`self.OwnerCharacter`))) (`KismetMathLibrary.Normal` (- (`Actor.K2_GetActorLocation` Interactble) (`Actor.K2_GetActorLocation` (`self.GetOwner`)))))) 120.0)))